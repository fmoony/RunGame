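; BP_DestructibleWall is a wall collision target meant to react to skill impacts, currently in a debug state.
; Its Impact event only prints the impact type tag, normal, instigator, point, direction, force and skill tag.
; The destruction logic, which disables collision, spawns the NS_Damage effect and hides WallMesh, is disconnected and never runs.
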(event EventBeginPlay)

(event Collision|EventActorBeginOverlap
  (params (OtherActor :type Actor%20Object%20Reference)))

(event EventTick
  (params (DeltaSeconds :type Float%20%28single-precision%29)))

(event EventImpact
  (params (SkillTag :type Gameplay%20Tag%20Structure) (Impact :type Impact%20Info%20Structure%20%28by%20ref%29))
  (Development|PrintString (GameplayTags|GetDebugStringfromGameplayTag (.impacttype Impact)) true true "(R=1.000000,G=0.660000,B=1.000000,A=1.000000)")
  (Development|PrintString (Utilities|String|ToString(Vector) (.impactnormal Impact)))
  (Development|PrintString (Utilities|GetDisplayName (.instigator Impact)))
  (Development|PrintString (Utilities|String|ToString(Vector) (.impactpoint Impact)))
  (Development|PrintString (Utilities|String|ToString(Vector) (.direction Impact)))
  (Development|PrintString (Utilities|String|ToString(Float) (.force Impact)))
  (Development|PrintString (GameplayTags|GetDebugStringfromGameplayTag SkillTag) true true "(R=1.000000,G=0.000000,B=0.127381,A=1.000000)"))

(fn ConstructionScript)