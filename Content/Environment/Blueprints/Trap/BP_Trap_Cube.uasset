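; BP_Trap_Cube is a cube trap that switches on and off with the floor it belongs to.
; On BeginPlay it casts its parent actor to FloorBase and binds handlers to floor activation and deactivation, which call ActivateTrap and DeactivateTrap.
; EndPlay unbinds separate Release events rather than the bound handlers, so the original bindings are not removed by those calls.
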(event Custom|Handle_OnFloorActivated
  (params (Floor :type Floor%20Base%20Object%20Reference))
  (Class|Trap|ActivateTrap self))

(event Custom|Handle_OnFloorDeactivated
  (params (Floor :type Floor%20Base%20Object%20Reference))
  (Class|Trap|DeactivateTrap self))

(event Custom|Release_OnFloorActivated
  (params (Floor :type Floor%20Base%20Object%20Reference))
  (Class|Trap|ActivateTrap self))

(event Custom|Release_OnFloorDeactivated
  (params (Floor :type Floor%20Base%20Object%20Reference))
  (Class|Trap|DeactivateTrap self))

(event EventBeginPlay
  (bind _asfloor_base (Utilities|Casting|CastToFloorBase (Actor|GetParentActor self)))
  (EventDispatchers|BindEventtoOnFloorActivated _asfloor_base (delegate Custom|Handle_OnFloorActivated))
  (EventDispatchers|BindEventtoOnFloorDeactivated _asfloor_base (delegate Custom|Handle_OnFloorDeactivated)))

(event EventEndPlay
  (params (EndPlayReason :type EEndPlayReason%20Enum :default "Destroyed"))
  (bind _asfloor_base (Utilities|Casting|CastToFloorBase (Actor|GetParentActor self)))
  (EventDispatchers|UnbindEventfromOnFloorActivated _asfloor_base (delegate Custom|Release_OnFloorActivated))
  (EventDispatchers|UnbindEventfromOnFloorDeactivated _asfloor_base (delegate Custom|Release_OnFloorDeactivated)))

(fn ConstructionScript)